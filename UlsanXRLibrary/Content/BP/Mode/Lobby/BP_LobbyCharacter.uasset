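; Lobby player character Blueprint that sets up networked voice chat through a VOIPTalker component.
; BeginPlay waits briefly, then starts networked voice if the talker is valid.
; InitVOIPComp retries on a short delay until PlayerState is valid, then registers the talker, sets mic threshold and attaches voice to the capsule.
; It then calls VoiceSetting, which tunes mic gain and noise thresholds through console commands for the locally controlled player.
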(event Custom|VoiceSetting
  (bind _returnvalue (Game|GetPlayerController 0))
  ;[0.15 0.15 0.15 0.5 106] 음성 세팅
  (if (Pawn|IsLocallyControlled)
    (Development|ExecuteConsoleCommand "voice.MicInputGain 5" _returnvalue)
    (Development|ExecuteConsoleCommand "voice.MicNoiseGateThreshold 0.02" _returnvalue)
    (Development|ExecuteConsoleCommand "voice.SilenceDetectionThreshold 0.02" _returnvalue)))

(event Custom|InitVOIPComp
  (bind _playerstate (Variables|Default|GetPlayerState))
  ;[0.15 0.15 0.15 0.5 74] VOIP 붙이기
  (Utilities|IsValid _playerstate :!label _label
    (:Is%20Valid
      (Class|VOIPTalker|RegisterwithPlayerState (Variables|Default|GetVOIPTalker) _playerstate)
      (Class|VOIPStatics|SetMicThreshold 0.2)
      (Variables|/Script/Engine.VOIPTalker|SetSettings (Variables|Default|GetVOIPTalker) (Utilities|Struct|MakeVoiceSettings (Variables|Default|GetCapsuleComponent) 0 0))
      (CallFunction|VoiceSetting)
      (Development|PrintString "Voice Session"))
    (:Is%20Not%20Valid
      (Utilities|FlowControl|Delay 0.1)
      (goto _label))))

(event EventBeginPlay
  (Development|PrintString "Lobby Character")
  (Utilities|FlowControl|Delay 3.0)
  (Variables|Default|GetVOIPTalker
    (:then
      (Class|AdvancedVoiceLibrary|StartNetworkedVoice))
    (:else)))

(event Collision|EventActorBeginOverlap
  (params (OtherActor :type Actor%20Object%20Reference))
  ;[0.15 0.15 0.15 0.5 106] 음성 세팅
)

(event EventTick
  (params (DeltaSeconds :type Float%20%28single-precision%29)))

(fn ConstructionScript)